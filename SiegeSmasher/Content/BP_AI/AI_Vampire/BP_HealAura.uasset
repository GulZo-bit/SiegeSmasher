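; BP_HealAura is a visual heal aura actor in the Vampire AI folder that shows a light effect when spawned.
; On BeginPlay, a timeline's fade-in-and-out track drives the intensity of inner and outer lights, then sets both to zero when it finishes.
; The graph contains no healing logic and does not destroy the actor afterwards.
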(event EventBeginPlay
  (bind _fadeinandout (Timeline|HealTimeLine PlayFromStart)
    (:Update
      (Variables|Default|SetNewVar (Variables|Default|GetHealTimeLine))
      (Rendering|Components|Light|SetIntensity (Variables|Default|GetHealLightInner) _fadeinandout)
      (Rendering|Components|Light|SetIntensity (Variables|Default|GetHealLightOuter) _fadeinandout))
    (:Finished
      (Rendering|Components|Light|SetIntensity (Variables|Default|GetHealLightOuter) 0.0)
      (Rendering|Components|Light|SetIntensity (Variables|Default|GetHealLightInner) 0.0))))

(event Collision|EventActorBeginOverlap
  (params (OtherActor :type Actor%20Object%20Reference)))

(event EventTick
  (params (DeltaSeconds :type Float%20%28single-precision%29)))

(fn ConstructionScript)